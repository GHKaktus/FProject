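; BP_Door is a level door that rises only while both the left and right buttons report open.
; On BeginPlay it stores its mesh's world location, finds BP_Button_Left and BP_Button_Right by class, and binds to their open and close dispatchers.
; Each event updates that side's flag; when both are set, MoveComponentTo lifts the mesh over time.
; Either close event sends it back to the stored location.
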(event `self.ReceiveBeginPlay`
  (bind _output_get (set `self.Down Location` (`SceneComponent.K2_GetComponentLocation` (`self.StaticMeshComponent`))))
  (bind _returnvalue (`GameplayStatics.GetActorOfClass` "/Game/Level/BP_Button_Left.BP_Button_Left_C"))
  (bind _output_get_2 (set `self.Button Left Ref` _returnvalue))
  (bind _returnvalue_2 (`GameplayStatics.GetActorOfClass` "/Game/Level/BP_Button_Right.BP_Button_Right_C"))
  (bind _output_get_3 (set `self.Button Right Ref` _returnvalue_2))
  (add `/Game/Level/BP_Button_Right.OpenRight` _output_get_3 (delegate `OpenRight`))
  (add `/Game/Level/BP_Button_Left.OpenLeft` _output_get_2 (delegate `OpenLeft`))
  (add `/Game/Level/BP_Button_Right.CloseRight` _output_get_3 (delegate `CloseRight`))
  (add `/Game/Level/BP_Button_Left.CloseLeft` _output_get_2 (delegate `CloseLeft`)))

(event `CloseRight`
  (set `self.Right Open` false)
  (`KismetSystemLibrary.MoveComponentTo` (`self.StaticMeshComponent`) (stale `self.ReceiveBeginPlay` _output_get) (struct) false false 1.0 :!label _label))

(event `OpenRight`
  (bind _output_get (set `self.Right Open` true))
  (if (and _output_get (stale `OpenLeft` _output_get)) :!label _label_2
    (`KismetSystemLibrary.MoveComponentTo` (`self.StaticMeshComponent`) (+ (stale `self.ReceiveBeginPlay` _output_get) (0.0 0.0 500.0)) (struct) false false 1.0)))

(event `CloseLeft`
  (set `self.Left Open` false)
  (goto _label))

(event `OpenLeft`
  (bind _output_get (set `self.Left Open` true))
  (goto _label_2))

(fn `UserConstructionScript`)